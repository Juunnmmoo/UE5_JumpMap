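; BP_Monster is an orbiting obstacle that knocks characters away on contact.
; At BeginPlay it moves the SM_Bottington component out along world X by Radios, then spins the whole actor in yaw each Tick at Speed, so the component circles the actor's origin.
; When that component hits a BF_Character, it launches the character along the negated hit normal with a fixed strength.
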(event `self.ReceiveBeginPlay`
  (bind (_returnvalue_x _returnvalue_y _returnvalue_z) (`KismetMathLibrary.BreakVector` (`self.K2_GetActorLocation`)))
  (`SceneComponent.K2_SetWorldLocation` (`self.SM_Bottington`) (`KismetMathLibrary.MakeVector` (+ (`self.Radios`) _returnvalue_x) _returnvalue_y _returnvalue_z) false false))

(event `self.ReceiveTick`
  (params (DeltaSeconds :type "Float (single-precision)"))
  (`self.K2_AddActorLocalRotation` (`KismetMathLibrary.MakeRotator` 0.0 0.0 (* (`self.Speed`) DeltaSeconds))))

(event `self.SM_Bottington.OnComponentHit`
  (params (HitComponent :type "PrimitiveComponent Object Reference") (OtherActor :type "Actor Object Reference") (OtherComp :type "PrimitiveComponent Object Reference") (NormalImpulse :type "Vector Structure") (Hit :type "HitResult Structure (by ref)"))
  (bind _asbf_character (cast `/Game/momoEngine/Blueprints/BF_Character` OtherActor))
  (`Character.LaunchCharacter` _asbf_character (* Hit_Normal (`KismetMathLibrary.Conv_DoubleToVector` -5000.0)) false false))

(fn `UserConstructionScript`)